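; Player pawn that reads text lines from a serial COM port and fires missiles on a key press.
; BeginPlay opens and flushes a UART connection on a fixed port, and Tick prints each line read, re-running the open step when the connection is invalid or a read fails.
; The Launch_key input spawns a scaled-down BP_Missile at the pawn's location and rotation, and EndPlay closes the port.
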(event `self.ReceiveBeginPlay`
  (bind (_bopened _returnvalue) (`SerialCom.OpenComPort` 8 :!label _label))
  (if _bopened
    (bind _output_get (set `self.UART_obj` _returnvalue))
    (`SerialCom.Flush` _output_get)
    (else
      (`KismetSystemLibrary.PrintText` (`KismetTextLibrary.Conv_BoolToText` _bopened))
      (`KismetSystemLibrary.PrintText` "Port"))))

(event `self.ReceiveTick`
  (params (DeltaSeconds :type "Float (single-precision)"))
  (bind _uart_obj (`self.UART_obj`))
  (`/Engine/EditorBlueprintResources/StandardMacros.IsValid` _uart_obj
    (:`Is Valid`
      (bind (_bsuccess _returnvalue) (`SerialCom.Readln` _uart_obj))
      (if _bsuccess
        (`KismetSystemLibrary.PrintString` _returnvalue)
        (else
          (`KismetSystemLibrary.PrintString` "Bad_read")
          (goto _label))))
    (:`Is Not Valid`
      (`KismetSystemLibrary.PrintString` "Try reopen port")
      (goto _label))))

(event `InputAction|Launch_key`
  (params (Key :type "Key Structure"))
  (:`Pressed`
    (`|SpawnActorFromClass` "/Game/BP_Missile.BP_Missile_C" (`KismetMathLibrary.MakeTransform` (`self.K2_GetActorLocation`) (`self.K2_GetActorRotation`) (0.4 0.4 0.4)) "Undefined" "OverrideRootScale" null null)))

(event `self.ReceiveEndPlay`
  (params (EndPlayReason :type "EEndPlayReason Enum" :default "Destroyed"))
  (bind _uart_obj (`self.UART_obj`))
  (`/Engine/EditorBlueprintResources/StandardMacros.IsValid` _uart_obj
    (:`Is Valid`
      (`SerialCom.Close` _uart_obj))))

(fn `UserConstructionScript`)