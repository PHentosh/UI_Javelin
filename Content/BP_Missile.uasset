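; BP_Missile is a missile actor that launches itself as soon as it begins play.
; BeginPlay calls a Launch function, defined outside this file, with fixed velocity components along negative X and upward Z.
; The remaining graph is leftover debug logic that never runs, printing rotation values and a flipped roll angle, plus unused multiplications.
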(event `self.ReceiveBeginPlay`
  (`self.Launch` -9800.0 0.0 3000.0))

(fn `UserConstructionScript`)